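; Quest system component that creates quests from DT_Quests by enum, keeps their live state in a Quests array and builds the quest panel and hotbar widgets.
; Task stage changes reveal the next task and complete or fail the quest from required tasks; missing quests are auto-created.
; When a tracked quest ends, another in-progress one gets tracked.
; SaveQuests stores the array; LoadQuests rebuilds widgets, refreshing text from the table.
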(event Custom|CheckNewTrackEvent
  (params (Delay :type Float%20%28single-precision%29))
  ;[0.1562 0.1562 0.1562] A slight delay before finding a new quest to track so the player has time to understand what is going on
  (Utilities|FlowControl|Delay Delay)
  (HUD|CheckNewTrack))

(event EventBeginPlay
  (Utilities|FlowControl|Sequence
    (:then_0
      ;[0.03125 0.03125 0.03125] Create Quest Panel Widget and init self reference
      ; -You can create your own widget with similar functionality or use this one as a template
      (bind _returnvalue (UserInterface|CreateWidget "/Game/QuestStartup/Blueprints/Widgets/WB_QuestsPanel.WB_QuestsPanel_C" 0 self))
      (bind _output_get (Variables|Default|SetQuestWidget _returnvalue))
      (UserInterface|Viewport|AddtoViewport _output_get 1)
      (Widget|SetVisibility _output_get "Hidden"))
    (:then_1
      ;[0.1198 0.09135 0.03303] Quest Hotbar to display tasks of the quest being tracked in the corner of the screen. You can add WB_TasksList to your Hotbar if you need it and provide its link here
      (bind _returnvalue_2 (UserInterface|CreateWidget "/Game/QuestStartup/Blueprints/Widgets/WB_QuestHotbar.WB_QuestHotbar_C"))
      (Variables|Default|SetHotbarTaskListWidget (Variables|/Game/QuestStartup/Blueprints/Widgets/WB_QuestHotbar.WB_QuestHotbar_C|GetWB_TasksList _returnvalue_2)) ; You need init this variable
      (UserInterface|Viewport|AddtoViewport _returnvalue_2 0))
    (:then_2
      ;[0.03125 0.03125 0.03125] [EXAMPLE] Сreate the first quest, which will be available immediately, without message
      ; You can create quests from anywhere as long as you have access to the Quest Component.
      (CallFunction|CreateQuest "NewEnumerator0" false))))

(fn GetQuestRefforEnum
  (params (QuestEnum :type E_Quests%20Enum :default "NewEnumerator0"))
  ;[0.005208 0.005208 0.005208] Search for a quest reference from existing quests
  (for (_array_element _array_index) (Variables|Default|GetQuests)
    (if (Utilities|Enum|Equal(Enum) (.QuestEnum (Utilities|Struct|BreakS_Quest _array_element)) QuestEnum)
      (return _array_element _array_index true)))
  (return "" 0 false))

(fn CreateQuest
  (params (QuestEnum :type E_Quests%20Enum :default "NewEnumerator0") (WithMessage :type Boolean))
  ;[0.01 0.01 0.01] Сreate a quest only if it has not been received yet
  (if (not (.Ok? (Info|GetQuestRefforEnum QuestEnum)))
    (bind _output_get (LocalVariables|SetQuestInfoLocal (Info|GetQuestDataforEnum QuestEnum)))
    ;[0.01 0.01 0.01] Create Quest widget in Widget Panel
    (bind _questwidget (Default|AddNewQuestWidget (Variables|Default|GetQuestWidget) _output_get))
    ;[0.01 0.01 0.01] Add quest widget reference to Quest Info
    (bind _structout (Utilities|Struct|SetmembersinS_Quest (LocalVariables|GetQuestInfoLocal) _questwidget))
    ;[0.01 0.01 0.01] Add New Quest info in Quest Array
    (bind _returnvalue (Utilities|Array|Add (Variables|Default|GetQuests) _structout))
    (LocalVariables|SetLocalIndex _returnvalue)
    (Utilities|FlowControl|Sequence
      (:then_0
        ;[0.08854 0.08854 0.08854] Сreate a simple message about receiving a new quest
        (if WithMessage
          (Variables|Default|SetLastGettedQuest QuestEnum)
          (HUD|CreatetoTrackMessage)))
      (:then_1
        ;[0.07812 0.07812 0.07812] Check if we can make a new quest for tracking
        (HUD|CheckNewTrack)
        (return (LocalVariables|GetLocalIndex) (LocalVariables|GetQuestInfoLocal))))))

(fn GetQuestDataforEnum
  (params (QuestEnum :type E_Quests%20Enum :default "NewEnumerator0"))
  ;[0.07292 0.07292 0.07292] Get Quest Info from Quests Data Table. It does not contain up-to-date information. It does not contain current relevant information about the quest, but is needed to create/initialize it.
  (bind _outrownames (DataTable|GetDataTableRowNames "/Game/QuestStartup/Blueprints/QuestSystem/DT_Quests.DT_Quests"))
  (for _array_element _outrownames
    (bind _returnvalue (Utilities|GetDataTableRow "/Game/QuestStartup/Blueprints/QuestSystem/DT_Quests.DT_Quests" _array_element)
      (:then
        (if (Utilities|Enum|Equal(Enum) (.QuestEnum (Utilities|Struct|BreakS_Quest _returnvalue)) QuestEnum)
          (return _returnvalue)))))
  (return ""))

(fn NewStageQuest
  (params (QuestEnum :type E_Quests%20Enum :default "NewEnumerator0") (NewStage :type E_QuestStage%20Enum :default "NewEnumerator0") (WithMessage :type Boolean))
  (bind (_questinfo _questindex _ok_) (Info|GetQuestRefforEnum QuestEnum))
  (if _ok_
    ;[0.01042 0.01042 0.01042] Array Update
    (bind _structout (Utilities|Struct|SetmembersinS_Quest (Utilities|Array|Get(acopy) (Variables|Default|GetQuests) _questindex) NewStage))
    (bind _output_get (LocalVariables|SetLocalInfo _structout))
    ;[0.02083 0.02083 0.02083] HUD Update
    (Default|NewQuestStage (.QuestWidgetRef (Utilities|Struct|BreakS_Quest _output_get)) NewStage)
    (LocalVariables|SetLocalName (.Name (Utilities|Struct|BreakS_Quest _output_get)))
    (Utilities|FlowControl|Sequence
      (:then_0
        ;[0.01562 0.01562 0.01562] Additional
        ;;[0.08854 0.08854 0.08854] Сreate a simple self-destructing message
        (if WithMessage
          (HUD|CreateSimpleMessage (Utilities|Select :Index NewStage :NewEnumerator0 (Utilities|Text|FormatText "Quest {0} in process!" (LocalVariables|GetLocalName)) :NewEnumerator1 (Utilities|Text|FormatText "Quest {0} is complete!" (LocalVariables|GetLocalName)) :NewEnumerator2 (Utilities|Text|FormatText "Quest {0} is Failed :(" (LocalVariables|GetLocalName))))))
      (:then_1
        ;;[0.1094 0.1094 0.1094] If the quest is complete or failed, find a new quest to track
        (if (not (Utilities|Enum|Equal(Enum) NewStage "NewEnumerator0"))
          (CallFunction|CheckNewTrackEvent 2.0) ; We leave a small delay to give time to get acquainted with the stage of the previous quest
        ))
      (:then_2
        ;;[0.05208 0.05208 0.05208] Update the HUD, if the quests don't use tasks, we still need to update the color
        (if (.IsTracked (Utilities|Struct|BreakS_Quest (LocalVariables|GetLocalInfo)))
          (Default|RefreshTaskList (Variables|Default|GetHotbarTaskListWidget) (LocalVariables|GetLocalInfo) true))))))

(fn CreateSimpleMessage
  (params (TextMessage :type Text))
  ;[0.04688 0.04688 0.04688] Сreate a simple self-destructing message
  (bind _returnvalue (UserInterface|CreateWidget "/Game/QuestStartup/Blueprints/Widgets/Additional/WB_Message.WB_Message_C" 0 TextMessage))
  (UserInterface|Viewport|AddtoViewport _returnvalue 0))

(fn SetQuestNotification
  (params (Quest :type E_Quests%20Enum :default "NewEnumerator0") (QuestWidgetRef :type WB%20Quest%20Object%20Reference) (Notify :type Boolean))
  (bind (_questinfo _questindex _ok_) (Info|GetQuestRefforEnum Quest))
  ;[0.02604 0.02604 0.02604] Change the current state of the notification (orange circle). It is displayed only in the widget, but we need to store its state, for example, for the save system
  (if _ok_
    ;;[0.04167 0.04167 0.04167] When using "set members" do not forget to take the array [get a ref] (blue rhombus)
    (Utilities|Struct|SetmembersinS_Quest (Utilities|Array|Get(acopy) (Variables|Default|GetQuests) _questindex) Notify)
    ;[0.03646 0.03646 0.03646] Update HUD
    (Default|SetNotify QuestWidgetRef Notify)))

(fn NewQuestTracked
  (params (QuestEnum :type E_Quests%20Enum :default "NewEnumerator0") (IsTracked :type Boolean))
  (bind (_questinfo _questindex _ok_) (Info|GetQuestRefforEnum QuestEnum))
  (bind _hotbartasklistwidget (Variables|Default|GetHotbarTaskListWidget))
  ;[1 1 1] Untrack all quests
  (for (_array_element _array_index) (Variables|Default|GetQuests)
    (bind _structout (Utilities|Struct|SetmembersinS_Quest _array_element false))
    (Utilities|Array|SetArrayElem (Variables|Default|GetQuests) _array_index _structout true))
  ;[1 1 1] Track need quest if IsTracked = True, else Hidden TaskListWidget
  (if (and _ok_ IsTracked)
    (bind _structout_2 (Utilities|Struct|SetmembersinS_Quest (Utilities|Array|Get(acopy) (Variables|Default|GetQuests) _questindex) true))
    (Default|RefreshTaskList _hotbartasklistwidget _structout_2 true)
    (Widget|SetVisibility _hotbartasklistwidget "Visible")
    (else
      (Widget|SetVisibility (Variables|Default|GetHotbarTaskListWidget) "Hidden"))))

(fn NewStageTask
  (params (Quest :type E_Quests%20Enum :default "NewEnumerator0") (NumTask :type Integer) (NewStage :type E_QuestStage%20Enum :default "NewEnumerator1") (ShowNextTask :type Boolean))
  (bind (_questinfo _questindex _ok_) (Info|GetQuestRefforEnum Quest))
  (bind _quests (Variables|Default|GetQuests))
  (bind _output (Utilities|Array|Get(acopy) _quests _questindex))
  (bind _returnvalue (+ NumTask 1))
  (bind (_questenum _name _description _stageofcompletion _notification _tasks _questwidgetref) (Utilities|Struct|BreakS_Quest _output))
  ;[0.04688 0.04688 0.04688] Update Task stage in quest
  (LocalVariables|SetLocalIndex _questindex) ; Helper local variable
  (if _ok_
    (LocalVariables|SetQuestWidgetLocal _questwidgetref) ; Helper local variable
    (if (Utilities|Array|IsValidIndex _tasks NumTask)
      (Utilities|Struct|SetmembersinS_QuestTask (Utilities|Array|Get(acopy) _tasks NumTask) NewStage true) ; when changing the stage we set visibility true\neven if the task has not yet been received, since the player can complete it earlier
      (Utilities|FlowControl|Sequence
        (:then_0
          ;[0.06771 0.06771 0.06771] We check whether all the required tasks of the quest have been completed
          (bind _changequeststage (Helper|AllQuestTasksCompleted? Quest))
          (if (not _changequeststage)
            ;[0.04688 0.04688 0.04688] show task status message if quest status message is not called
            (HUD|CreateSimpleMessage (Utilities|Select :Index NewStage :NewEnumerator0 "Task In progress!" :NewEnumerator1 "Task is complete!" :NewEnumerator2 "Task is complete!"))))
        (:then_1
          ;[0.03646 0.03646 0.03646] Automatically display the next task if there is one, if the current task has been completed or failed
          (if (Math|Boolean|ANDBoolean ShowNextTask (Utilities|Array|IsValidIndex (.Tasks (Utilities|Struct|BreakS_Quest (Utilities|Array|Get(acopy) (Variables|Default|GetQuests) (LocalVariables|GetLocalIndex)))) _returnvalue) (not (Utilities|Enum|Equal(Enum) NewStage "NewEnumerator0")))
            (CallFunction|SetVisibleTask (.QuestEnum (Utilities|Struct|BreakS_Quest (Utilities|Array|Get(acopy) (Variables|Default|GetQuests) (LocalVariables|GetLocalIndex)))) _returnvalue true)
            (else
              ;[0.05729 0.05729 0.05729] If the SetVisibleTask function was not called, update the HUD here
              (HUD|HUDTasksUpdate Quest)))))
      (else
        (CallFunction|NewStageQuest Quest NewStage false) ; If there is no task with such index, transfer this stage to the quest
      ))
    (else
      ;;[0.07292 0.07292 0.07292] if the quest has not yet been received
      (CallFunction|CreateQuest Quest true)
      (CallFunction|NewStageTask Quest NumTask NewStage ShowNextTask))))

(fn AllQuestTasksCompleted?
  (params (QuestEnum :type E_Quests%20Enum :default "NewEnumerator0"))
  (bind (_questinfo _questindex _ok_) (Info|GetQuestRefforEnum QuestEnum))
  ;[0.1042 0.1042 0.1042] We check if all the quest required tasks are completed, if so, we make the quest complete.
  ; If at least one of the required tasks fails, then the entire quest fails
  (if _ok_
    (for _array_element (.Tasks (Utilities|Struct|BreakS_Quest _questinfo))
      (if (.IsRequired (Utilities|Struct|BreakS_QuestTask _array_element))
        (if (not (Utilities|Enum|Equal(Enum) (.TaskStage (Utilities|Struct|BreakS_QuestTask _array_element)) "NewEnumerator2")) ; If at least one of the required tasks fails, then the entire quest fails
          (LocalVariables|SetCompleteLocal (and (Utilities|Enum|Equal(Enum) (.TaskStage (Utilities|Struct|BreakS_QuestTask _array_element)) "NewEnumerator1") (LocalVariables|GetCompleteLocal)))
          (else
            (CallFunction|NewStageQuest QuestEnum "NewEnumerator2" true)
            (return true)))))
    (if (LocalVariables|GetCompleteLocal)
      (CallFunction|NewStageQuest QuestEnum "NewEnumerator1" true)
      (return true)
      (else
        (return false)))))

(fn SetVisibleTask
  (params (QuestEnum :type E_Quests%20Enum :default "NewEnumerator0") (NumTask :type Integer) (IsVisble :type Boolean))
  (bind (_questinfo _questindex _ok_) (Info|GetQuestRefforEnum QuestEnum))
  ;[0.125 0.125 0.125] Toggles the visibility of the a new task in the quest
  (if _ok_
    (Utilities|Struct|SetmembersinS_QuestTask (Utilities|Array|Get(acopy) (.Tasks (Utilities|Struct|BreakS_Quest (Utilities|Array|Get(acopy) (Variables|Default|GetQuests) _questindex))) NumTask) IsVisble)
    ;[0.05729 0.05729 0.05729] Update HUD with new info
    (HUD|HUDTasksUpdate QuestEnum)
    (else
      ;;[0.05729 0.05729 0.05729] If the quest has not been created yet, create it and call the same function
      (CallFunction|CreateQuest QuestEnum true)
      (CallFunction|SetVisibleTask QuestEnum NumTask IsVisble))))

(fn HUDTasksUpdate
  (params (Quest :type E_Quests%20Enum :default "NewEnumerator0"))
  (bind (_questinfo _questindex _ok_) (Info|GetQuestRefforEnum Quest))
  (if _ok_
    (LocalVariables|SetLocalQuestInfo _questinfo)
    (Utilities|FlowControl|Sequence
      (:then_0
        ;[0.09375 0.08786 0.05699] HUD Update
        ;;[0.05729 0.05729 0.05729] Update task description if this quest is already open in the quest widget
        (if (Variables|/Game/QuestStartup/Blueprints/Widgets/Additional/WB_Quest.WB_Quest_C|GetIsReading? (.QuestWidgetRef (Utilities|Struct|BreakS_Quest (LocalVariables|GetLocalQuestInfo))))
          (Default|RefreshTasks (Variables|Default|GetQuestWidget) (LocalVariables|GetLocalQuestInfo))))
      (:then_1
        ;;[0.09701 0.07268 0.09896] Refresh the task list in the hotbar if this quest is currently being tracked
        (if (and (Widget|IsVisible (Variables|Default|GetHotbarTaskListWidget)) (.IsTracked (Utilities|Struct|BreakS_Quest (LocalVariables|GetLocalQuestInfo))))
          (Default|RefreshTaskList (Variables|Default|GetHotbarTaskListWidget) (LocalVariables|GetLocalQuestInfo) true)))
      (:then_2
        ;;[0.09375 0.09375 0.09375] Add notification updated quest
        (HUD|SetQuestNotification (.QuestEnum (Utilities|Struct|BreakS_Quest (LocalVariables|GetLocalQuestInfo))) (.QuestWidgetRef (Utilities|Struct|BreakS_Quest (LocalVariables|GetLocalQuestInfo))) true)))))

(fn CheckNewTrack
  (bind (_questenum _ok_) (Helper|GetTrackedQuest))
  ;[0.06771 0.06771 0.06771] Find for a new quest to track if possible
  (if _ok_
    ;;[0.1979 0.1979 0.1979] If the quest being tracked is already completed or failed
    (if (not (Utilities|Enum|Equal(Enum) (.StageOfCompletion (Utilities|Struct|BreakS_Quest (.QuestInfo (Info|GetQuestRefforEnum _questenum)))) "NewEnumerator0"))
      ;;[0.0625 0.0625 0.0625] If no quest is tracked, then we track the first one found
      (for _array_element (Variables|Default|GetQuests) :!label _label
        (if (Utilities|Enum|Equal(Enum) (.StageOfCompletion (Utilities|Struct|BreakS_Quest _array_element)) "NewEnumerator0")
          (HUD|NewQuestTracked (.QuestEnum (Utilities|Struct|BreakS_Quest _array_element)) true)
          (return))))
    (else
      (goto _label))))

(fn GetTrackedQuest
  (for _array_element (Variables|Default|GetQuests)
    (if (.IsTracked (Utilities|Struct|BreakS_Quest _array_element))
      (return (.QuestEnum (Utilities|Struct|BreakS_Quest _array_element)) true)))
  (return "NewEnumerator0" false))

(fn CreatetoTrackMessage
  ;[0.04688 0.04688 0.04688] Сreate a simple self-destructing message
  (bind _returnvalue (UserInterface|CreateWidget "/Game/QuestStartup/Blueprints/Widgets/Additional/WB_TrackQuestMessage.WB_TrackQuestMessage_C"))
  (UserInterface|Viewport|AddtoViewport _returnvalue 0))

(fn SaveQuests
  ;[0.09375 0.09375 0.09375] Example of simple saving
  (bind _returnvalue (SaveGame|CreateSaveGameObject "/Game/QuestStartup/Blueprints/SaveLoad/BP_SaveGame.BP_SaveGame_C"))
  (bind _output_get (LocalVariables|SetLocalSaveGame _returnvalue))
  (Variables|/Game/QuestStartup/Blueprints/SaveLoad/BP_SaveGame.BP_SaveGame_C|SetQuests _output_get (Variables|Default|GetQuests))
  (SaveGame|SaveGametoSlot (LocalVariables|GetLocalSaveGame) "default"))

(fn LoadQuests
  ;[0.2083 0.2057 0.09147] Getting saved quest state from save slot. (You can change this to your logic to get the stored array)
  (bind _returnvalue (SaveGame|LoadGamefromSlot "default"))
  (bind _asbp_save_game (Utilities|Casting|CastToBP_SaveGame _returnvalue))
  (bind _output_get (Variables|Default|SetQuests (Variables|/Game/QuestStartup/Blueprints/SaveLoad/BP_SaveGame.BP_SaveGame_C|GetQuests _asbp_save_game)))
  ;[0.07292 0.07292 0.07292] Clearing the main quest panel
  (Default|ClearQuestWidgets (Variables|Default|GetQuestWidget))
  ;[0.05729 0.05729 0.05729] Load Logic
  (for (_array_element _array_index) _output_get
    (SaveLoad|LoadQuest _array_element _array_index)
    ;[0.03646 0.03646 0.03646] Track the quest if it was tracked at the time of saving
    (if (.IsTracked (Utilities|Struct|BreakS_Quest _array_element))
      (HUD|NewQuestTracked (.QuestEnum (Utilities|Struct|BreakS_Quest _array_element)) true))))

(fn LoadQuest
  (params (QuestInfo :type S%20Quest%20Structure) (ID :type Integer))
  (LocalVariables|SetLocalQuestInform QuestInfo)
  (Utilities|FlowControl|Sequence
    (:then_0
      ;[1 0.9257 0.4208] We update all the text to the current one from the Data Table. Because if we change the text of the quests, the old saves will remain with outdated data
      (bind _output_get (LocalVariables|SetTasksLocal (.Tasks (Utilities|Struct|BreakS_Quest (LocalVariables|GetLocalQuestInform)))))
      (for (_array_element _array_index) _output_get
        (Utilities|Struct|SetmembersinS_QuestTask _array_element (.TaskText (Utilities|Struct|BreakS_QuestTask (Utilities|Array|Get(acopy) (.Tasks (Utilities|Struct|BreakS_Quest (Info|GetQuestDataforEnum (.QuestEnum (Utilities|Struct|BreakS_Quest (LocalVariables|GetLocalQuestInform)))))) _array_index))) (.TextComplete (Utilities|Struct|BreakS_QuestTask (Utilities|Array|Get(acopy) (.Tasks (Utilities|Struct|BreakS_Quest (Info|GetQuestDataforEnum (.QuestEnum (Utilities|Struct|BreakS_Quest (LocalVariables|GetLocalQuestInform)))))) _array_index)))))
      (Utilities|Struct|SetmembersinS_Quest (LocalVariables|GetLocalQuestInform) (.Name (Utilities|Struct|BreakS_Quest (Info|GetQuestDataforEnum (.QuestEnum (Utilities|Struct|BreakS_Quest (LocalVariables|GetLocalQuestInform)))))) (.Description (Utilities|Struct|BreakS_Quest (Info|GetQuestDataforEnum (.QuestEnum (Utilities|Struct|BreakS_Quest (LocalVariables|GetLocalQuestInform)))))) (LocalVariables|GetTasksLocal)))
    (:then_1
      ;[0.01 0.01 0.01] Create Quest widget in Widget Panel
      (bind _questwidget (Default|AddNewQuestWidget (Variables|Default|GetQuestWidget) (LocalVariables|GetLocalQuestInform)))
      (bind _structout (Utilities|Struct|SetmembersinS_Quest (LocalVariables|GetLocalQuestInform) _questwidget))
      ;[0.01 0.01 0.01] Update the reference with relevant information
      (Utilities|Array|SetArrayElem (Variables|Default|GetQuests) ID _structout true))))

(fn GetSortedQuests
  (params (SortType :type E_QuestStage%20Enum :default "NewEnumerator0"))
  (for (_array_element _array_index) (Variables|Default|GetQuests)
    (if (Utilities|Enum|Equal(Enum) (.StageOfCompletion (Utilities|Struct|BreakS_Quest _array_element)) SortType)
      (Utilities|Map|Add (LocalVariables|GetLocalQuests) _array_index _array_element) ; Add quest info and specific main array[Quests] index
    ))
  (return (LocalVariables|GetLocalQuests)))