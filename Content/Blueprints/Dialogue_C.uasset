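; Dialogue Blueprint that feeds a cycling list of lines to the player character for display as speaking messages.
; When Speaking fires, it first checks that the player character has no speaking message active, then sends the current line along with the text delay.
; The index advances after each line and wraps to the first once the list runs out.
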(event Custom|Speaking
  (bind _returnvalue (Game|GetPlayerCharacter 0))
  (bind _dialogue (Variables|Default|GetDialogue))
  (bind _bspeaking (Class|PlayerBPI|CheckSpeaking(Message) _returnvalue))
  (if (not _bspeaking)
    (Class|PlayerBPI|Speaking(Message) _returnvalue (Utilities|Array|Get(acopy) _dialogue (Variables|Default|GetCurrentDialogue)) (Variables|Default|GetTextDelay))
    (bind _result (Math|Integer|IncrementInt (Variables|Default|GetCurrentDialogue))
      (:%20%20
        (if (>= _result (Utilities|Array|Length _dialogue))
          (Variables|Default|SetCurrentDialogue 0))))))